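; Player controller for the shooter that turns mouse movement into look input and stores separate sensitivities for mouse, touch and gyro.
; Mouse axes apply scaled yaw and pitch only while Mouse is the controlling device; touch and gyro input are not handled here.
; Getter and setter functions expose the active device and each device's sensitivity.
; Pressing G prints a test string, switches to UI-only input with a visible cursor and opens a sensitivity debug widget.
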(event EventBeginPlay)

(event EventTick
  (params (DeltaSeconds :type Float%20%28single-precision%29)))

(event Input|MouseEvents|MouseX
  (params (AxisValue :type Float%20%28single-precision%29))
  (if (Utilities|Enum|Equal(Enum) (Variables|Default|GetCurrentControllingDevice) "NewEnumerator0")
    (Class|PlayerController|AddYawInput (* AxisValue (Variables|Default|GetMouseSensitivityCurrent)))))

(event Input|MouseEvents|MouseY
  (params (AxisValue :type Float%20%28single-precision%29))
  (if (Utilities|Enum|Equal(Enum) (Variables|Default|GetCurrentControllingDevice) "NewEnumerator0")
    (Class|PlayerController|AddPitchInput (* AxisValue (Variables|Default|GetMouseSensitivityCurrent)))))

(event Input|MouseEvents|LeftMouseButton
  (params (Key :type Key%20Structure :default "AnyKey")))

(event Input|KeyboardEvents|G
  (params (Key :type Key%20Structure :default "AnyKey"))
  (:Pressed
    (Development|PrintString "Hello")
    (Input|SetInputModeUIOnly 0 0 true)
    (Variables|Default|SetbShowMouseCursor true)
    (bind _returnvalue (UserInterface|CreateWidget "/Game/WarPlanRed/Blueprints/UISensitivityDebug.UISensitivityDebug_C"))
    (UserInterface|Viewport|AddtoViewport _returnvalue 0)))

(fn ConstructionScript)

(fn GetCurrentControllingDevice
  (return (Variables|Default|GetCurrentControllingDevice)))

(fn SetCurrentControllingDevice
  (params (CurrentControllingDevice :type Controls%20Enum))
  (Variables|Default|SetCurrentControllingDevice CurrentControllingDevice))

(fn GetSensitivity
  (params (NewDevice :type Controls%20Enum) (CurrentDevice :type Boolean))
  (Utilities|FlowControl|Sequence
    (:then_0
      (if CurrentDevice
        (switch Utilities|FlowControl|Switch|SwitchonControls (Variables|Default|GetCurrentControllingDevice)
          (:NewEnumerator0
            (LocalVariables|SetLocalSensitivity (Variables|Default|GetMouseSensitivityCurrent)))
          (:NewEnumerator1
            (LocalVariables|SetLocalSensitivity (Variables|Default|GetTouchSensitivityCurrent)))
          (:NewEnumerator2
            (LocalVariables|SetLocalSensitivity (Variables|Default|GetGyroSensitivityCurrent))))
        (else
          (switch Utilities|FlowControl|Switch|SwitchonControls NewDevice
            (:NewEnumerator0
              (LocalVariables|SetLocalSensitivity (Variables|Default|GetMouseSensitivityCurrent)))
            (:NewEnumerator1
              (LocalVariables|SetLocalSensitivity (Variables|Default|GetTouchSensitivityCurrent)))
            (:NewEnumerator2
              (LocalVariables|SetLocalSensitivity (Variables|Default|GetGyroSensitivityCurrent)))))))
    (:then_1
      (return (LocalVariables|GetLocalSensitivity)))))

(fn SetSensitivity
  (params (New%20Device :type Controls%20Enum) (New%20Sensitivity :type Float%20%28single-precision%29))
  (switch Utilities|FlowControl|Switch|SwitchonControls New%20Device
    (:NewEnumerator0
      (Variables|Default|SetMouseSensitivityCurrent New%20Sensitivity))
    (:NewEnumerator1
      (Variables|Default|SetTouchSensitivityCurrent New%20Sensitivity))
    (:NewEnumerator2
      (Variables|Default|SetGyroSensitivityCurrent New%20Sensitivity))))