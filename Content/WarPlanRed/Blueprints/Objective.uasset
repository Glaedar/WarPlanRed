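; Objective is an unfinished flag capture point actor with a capture radius sphere and a movable flag.
; Tick prints a debug message when the sphere's overlap check passes, while the J key independently calls RaiseFlag.
; RaiseFlag increments CapturePercentage and, unless FlagCaptured, sets the flag's relative Z to a fixed offset rather than raising it progressively.
; LowerFlag is empty, and the overlap-driven capture logic is disconnected.
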(event `self.ReceiveTick`
  (params (DeltaSeconds :type "Float (single-precision)"))
  (if (`PrimitiveComponent.IsOverlappingActor` (`self.Sphere`) null)
    (`KismetSystemLibrary.PrintString` "Standing in Radius")))

(event `Key|J`
  (params (Key :type "Key Structure" :default "AnyKey"))
  (:`Pressed`
    (`self.RaiseFlag`)))

(fn `LowerFlag`)

(fn `RaiseFlag`
  (set `self.CapturePercentage` (+ (`self.CapturePercentage`) 1.0))
  (if (not (`self.FlagCaptured`))
    (`SceneComponent.K2_SetRelativeLocation` (`self.Flag`) (`KismetMathLibrary.MakeVector` 0.0 0.0 1.0) false false)))

(fn `UserConstructionScript`)