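; Test player character for a Wehrmacht soldier, with movement, sprinting, a fire-button flag and first/third-person views.
; First person uses separate body and legs meshes, hiding head and upper-spine bones respectively.
; LeftAlt toggles cameras, owner visibility and hand-socket attachment between views.
; Hard-coded keys also gate sprinting on holding W, swap the static mesh to an Stg50 and ragdoll the body.
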(event `self.ReceiveBeginPlay`
  (`|ExecutionSequence`
    (:`then_0`
      (`SkinnedMeshComponent.HideBoneByName` (`self.FP_Mesh`) "head" "PBO_None"))
    (:`then_1`
      (`SkinnedMeshComponent.HideBoneByName` (`self.FP_Legs`) "spine_03" "PBO_None"))))

(event `InputAxis|MoveForward`
  (params (AxisValue :type "Float (single-precision)"))
  (if (not (`self.DisableMovement`))
    (`self.AddMovementInput` (`KismetMathLibrary.GetForwardVector` (`KismetMathLibrary.MakeRotator` 0.0 0.0 (.yaw (`self.GetControlRotation`)))) AxisValue)))

(event `InputAxis|MoveSideways`
  (params (AxisValue :type "Float (single-precision)"))
  (if (not (`self.DisableMovement`))
    (`self.AddMovementInput` (`KismetMathLibrary.GetRightVector` (`KismetMathLibrary.MakeRotator` 0.0 0.0 (.yaw (`self.GetControlRotation`)))) AxisValue)))

(event `InputAction|Fire`
  (params (Key :type "Key Structure" :default "AnyKey"))
  (:`Pressed`
    (set `self.FiringButtonDown` true))
  (:`Released`
    (set `self.FiringButtonDown` false)))

(event `Key|LeftShift`
  (params (Key :type "Key Structure" :default "AnyKey"))
  (bind _charactermovement (`self.CharacterMovement`))
  ;[1 1 1] Sprinting
  (:`Pressed`
    (if (`self.Walking`)
      (set `self.SprintButtonDown` true)
      (set `CharacterMovementComponent.MaxWalkSpeed` (`self.SprintSpeed`) _charactermovement)))
  (:`Released`
    (set `self.SprintButtonDown` false)
    (set `CharacterMovementComponent.MaxWalkSpeed` (`self.WalkSpeed`) _charactermovement)))

(event `InputAction|ADS`
  (params (Key :type "Key Structure" :default "AnyKey")))

(event `Key|W`
  (params (Key :type "Key Structure" :default "AnyKey"))
  (:`Pressed`
    (set `self.Walking` true))
  (:`Released`
    (set `self.Walking` false)))

(event `Key|I`
  (params (Key :type "Key Structure" :default "AnyKey"))
  (:`Pressed`
    (`StaticMeshComponent.SetStaticMesh` (`self.StaticMesh`) "/Game/WarPlanRed/Meshes/Weapons/stg50.stg50")))

(event `Key|Y`
  (params (Key :type "Key Structure" :default "AnyKey"))
  (:`Pressed`
    (`PrimitiveComponent.AddImpulse` (`self.Mesh`) (0.0 0.0 10.0) "None" false)
    (`PrimitiveComponent.SetSimulatePhysics` (`self.Mesh`) true)
    (`PrimitiveComponent.SetCollisionProfileName` (`self.Mesh`) "Ragdoll")))

(event `Key|LeftAlt`
  (params (Key :type "Key Structure" :default "AnyKey"))
  (bind _fp_camera (`self.FP_Camera`))
  (bind _tp_camera (`self.TP_Camera`))
  (:`Pressed`
    (`/Engine/EditorBlueprintResources/StandardMacros.FlipFlop`
      (:`A`
        (`ActorComponent.SetActive` _tp_camera true false)
        (`ActorComponent.SetActive` _fp_camera false false)
        (`PrimitiveComponent.SetOwnerNoSee` (`self.Mesh`) false)
        (`PrimitiveComponent.SetOwnerNoSee` (`self.FP_Mesh`) true)
        (`PrimitiveComponent.SetOwnerNoSee` (`self.FP_Legs`) true)
        (`self.K2_AttachToComponent` (`self.Mesh`) "hand_l" "KeepRelative" "KeepRelative" "KeepRelative"))
      (:`B`
        (`ActorComponent.SetActive` _fp_camera true false)
        (`ActorComponent.SetActive` _tp_camera false false)
        (`PrimitiveComponent.SetOwnerNoSee` (`self.Mesh`) true)
        (`PrimitiveComponent.SetOwnerNoSee` (`self.FP_Mesh`) false)
        (`PrimitiveComponent.SetOwnerNoSee` (`self.FP_Legs`) false)
        (`self.K2_AttachToComponent` (`self.FP_Mesh`) "hand_l" "KeepRelative" "KeepRelative" "KeepRelative")))))

(fn `UserConstructionScript`)